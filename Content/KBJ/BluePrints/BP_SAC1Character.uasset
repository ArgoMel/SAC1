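; BP_SAC1Character is a character Blueprint that spawns and commands a friendly AI companion.
; On BeginPlay it spawns a BP_FriendlyAI behind and slightly below itself and stores the reference, printing a debug message if that fails.
; Hold, Follow and Recon input actions each set the companion's AIWork enum to a different state when the reference is valid.
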(event `self.ReceiveBeginPlay`
  (bind _location (.location (`self.GetTransform`)))
  (`KismetSystemLibrary.PrintString` (`KismetStringLibrary.Conv_VectorToString` _location))
  (bind _returnvalue (`|SpawnActorFromClass` "/Game/01_FriendlyAI/BP_FriendlyAI.BP_FriendlyAI_C" (`KismetMathLibrary.MakeTransform` (+ _location (* (`self.GetActorForwardVector`) -200.0) (0.0 0.0 -6.0)) (.rotation (`self.GetTransform`))) "AdjustIfPossibleButAlwaysSpawn" "MultiplyWithRoot" null null))
  (`/Engine/EditorBlueprintResources/StandardMacros.IsValid` _returnvalue
    (:`Is Valid`
      (set `self.FriendlyAI` _returnvalue))
    (:`Is Not Valid`
      (`KismetSystemLibrary.PrintString` "FriendlyAIFailCast"))))

(event `InputAction|Hold`
  (params (Key :type "Key Structure"))
  (bind _friendlyai (`self.FriendlyAI`))
  (:`Pressed`
    (`/Engine/EditorBlueprintResources/StandardMacros.IsValid` _friendlyai
      (:`Is Valid`
        (set `/Game/01_FriendlyAI/BP_FriendlyAI.AIWork` "NewEnumerator0" _friendlyai)))))

(event `InputAction|Follow`
  (params (Key :type "Key Structure"))
  (bind _friendlyai (`self.FriendlyAI`))
  (:`Pressed`
    (`/Engine/EditorBlueprintResources/StandardMacros.IsValid` _friendlyai
      (:`Is Valid`
        (set `/Game/01_FriendlyAI/BP_FriendlyAI.AIWork` "NewEnumerator1" _friendlyai)))))

(event `InputAction|Recon`
  (params (Key :type "Key Structure"))
  (bind _friendlyai (`self.FriendlyAI`))
  (:`Pressed`
    (`/Engine/EditorBlueprintResources/StandardMacros.IsValid` _friendlyai
      (:`Is Valid`
        (set `/Game/01_FriendlyAI/BP_FriendlyAI.AIWork` "NewEnumerator2" _friendlyai)))))

(fn `UserConstructionScript`)