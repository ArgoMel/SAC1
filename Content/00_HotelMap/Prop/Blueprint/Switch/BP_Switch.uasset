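; BP_Switch is a one-use interactable switch prop in the hotel map that unlocks the next actor in an interaction chain.
; Its Box overlap registers the switch as the SAC1 character's TriggerAct and stores that character, clearing TriggerAct on exit.
; Interacted calls Interaction, which, while CanUse is set, disables the switch, calls SetAIETC on the player and enables CanUse on NextInteractedActor if valid.
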(event `Interaction`
  (bind _nextinteractedactor (`self.NextInteractedActor`))
  (if (`self.CanUse`)
    (set `self.CanUse` false)
    (`/Game/KBJ/BluePrints/BP_SAC1Character.SetAIETC` (`self.Player`))
    (`/Engine/EditorBlueprintResources/StandardMacros.IsValid` _nextinteractedactor
      (:`Is Valid`
        (set `/Game/00_HotelMap/Prop/Blueprint/BP_InteractedActor.CanUse` true _nextinteractedactor)))))

(event `self.Box_0.OnComponentBeginOverlap`
  (params (OverlappedComponent :type "PrimitiveComponent Object Reference") (OtherActor :type "Actor Object Reference") (OtherComp :type "PrimitiveComponent Object Reference") (OtherBodyIndex :type Integer) (bFromSweep :type Boolean) (SweepResult :type "HitResult Structure (by ref)"))
  (bind _asbp_sac1character (cast `/Game/KBJ/BluePrints/BP_SAC1Character` OtherActor)
    (:`then`
      (set `/Game/KBJ/BluePrints/BP_SAC1Character.TriggerAct` self _asbp_sac1character)
      (set `self.Player` _asbp_sac1character))
    (:`CastFailed`
      (`KismetSystemLibrary.PrintString` "InteractedActerCharacterCastFail"))))

(event `self.Box_0.OnComponentEndOverlap`
  (params (OverlappedComponent :type "PrimitiveComponent Object Reference") (OtherActor :type "Actor Object Reference") (OtherComp :type "PrimitiveComponent Object Reference") (OtherBodyIndex :type Integer))
  (bind _asbp_sac1character (cast `/Game/KBJ/BluePrints/BP_SAC1Character` OtherActor)
    (:`then`
      (set `/Game/KBJ/BluePrints/BP_SAC1Character.TriggerAct` null _asbp_sac1character))
    (:`CastFailed`
      (`KismetSystemLibrary.PrintString` "InteractedActerCharacterCastFail"))))

(fn `Interacted`
  (`self.Interaction`))

(fn `UserConstructionScript`
  (`parent.UserConstructionScript`))