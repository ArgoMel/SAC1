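; BP_Door is an interactable hotel-map door that swings open and closed, gated by a CanOpen flag.
; Box overlap sets or clears the character's TriggerAct and shows or hides a HUD prompt chosen by open state.
; Interacted calls Interaction, which plays or reverses a timeline lerping door yaw to -90 degrees.
; DoorOpen plays as opening starts, DoorClose when closing finishes, and Doortab when opening is disallowed.
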(event `self.ReceiveBeginPlay`
  (`SceneComponent.K2_SetRelativeRotation` :`self` (`self.SM_Door_1`)))

(event `Interaction`
  (if (`self.CanOpen`)
    (if (`self.IsOpen`)
      (set `self.IsOpen` false)
      (bind (_direction `_새_트랙_0`) (`Timeline|타임라인` :!via `Reverse` :!label _label)
        (:`Update`
          (`SceneComponent.K2_SetRelativeRotation` (`self.SM_Door_1`) (`KismetMathLibrary.MakeRotator` 0.0 0.0 (`KismetMathLibrary.Lerp` 0.0 -90.0 `_새_트랙_0`)) false false))
        (:`Finished`
          (if (not (`self.IsOpen`))
            (`AudioComponent.Play` (`self.DoorClose`) 0.0))))
      (else
        (set `self.IsOpen` true)
        (`AudioComponent.Play` (`self.DoorOpen`) 0.0)
        (goto _label)))
    (else
      (`AudioComponent.Play` (`self.Doortab`) 0.0))))

(event `self.Box_0.OnComponentBeginOverlap`
  (params (OverlappedComponent :type "PrimitiveComponent Object Reference") (OtherActor :type "Actor Object Reference") (OtherComp :type "PrimitiveComponent Object Reference") (OtherBodyIndex :type Integer) (bFromSweep :type Boolean) (SweepResult :type "HitResult Structure (by ref)"))
  (bind _returnvalue (`PlayerController.GetHUD` (`GameplayStatics.GetPlayerController` 0)))
  (bind _asbp_sac1character (cast `/Game/KBJ/BluePrints/BP_SAC1Character` OtherActor))
  (set `/Game/KBJ/BluePrints/BP_SAC1Character.TriggerAct` self _asbp_sac1character)
  (if (`self.IsOpen`)
    (bind _assac1hud (cast `SAC1HUD` _returnvalue)
      (:`then`
        (`SAC1HUD.SetInteractionText` _assac1hud "Visible" (`self.Name_1`)))
      (:`CastFailed`
        (`KismetSystemLibrary.PrintString` "Interactedactor::HUDCasatFail" true true (struct :`G` 0.66 :`B` 1.0 :`A` 1.0) 10.0 :!label _label_2)))
    (else
      (bind _assac1hud_2 (cast `SAC1HUD` _returnvalue)
        (:`then`
          (`SAC1HUD.SetInteractionText` _assac1hud_2 "Visible" (`self.Name`)))
        (:`CastFailed`
          (goto _label_2))))))

(event `self.Box_0.OnComponentEndOverlap`
  (params (OverlappedComponent :type "PrimitiveComponent Object Reference") (OtherActor :type "Actor Object Reference") (OtherComp :type "PrimitiveComponent Object Reference") (OtherBodyIndex :type Integer))
  (bind _asbp_sac1character (cast `/Game/KBJ/BluePrints/BP_SAC1Character` OtherActor))
  (set `/Game/KBJ/BluePrints/BP_SAC1Character.TriggerAct` null _asbp_sac1character)
  (bind _assac1hud (cast `SAC1HUD` (`PlayerController.GetHUD` (`GameplayStatics.GetPlayerController` 0)))
    (:`then`
      (`SAC1HUD.SetInteractionText` _assac1hud "Collapsed" (`self.Name`)))
    (:`CastFailed`
      (goto _label_2))))

(fn `Interacted`
  (`self.Interaction`))

(fn `UserConstructionScript`
  (`parent.UserConstructionScript`))