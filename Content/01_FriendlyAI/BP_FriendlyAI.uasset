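; Friendly AI pawn that carries an assault rifle, fights its assigned target and explodes when it dies.
; BeginPlay attaches the spawned weapon and registers the pawn with CTR_AIController, while damage is passed to FriendlyAIState.
; Tick faces the movement direction, or aims at the target when the controller needs no move, setting an aim-space pitch.
; Fire shoots with a montage or, when out of ammo, reloads once the reload montage completes.
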(event `self.ReceiveAnyDamage`
  (params (Damage :type "Float (single-precision)") (DamageType :type "DamageType Object Reference") (InstigatedBy :type "Controller Object Reference") (DamageCauser :type "Actor Object Reference"))
  (`/Game/01_FriendlyAI/FriendlyAIState.SetHP` (`self.FriendlyAIState`) (`KismetMathLibrary.FTrunc` Damage)))

(event `self.ReceiveBeginPlay`
  (set `self.AIWork` "NewEnumerator0")
  (bind _returnvalue (`|SpawnActorFromClass` "/Game/02_Gun/Riffle/BP_Weapon_AssaultRifle.BP_Weapon_AssaultRifle_C" (`self.Spawn Transform`) "Undefined" "MultiplyWithRoot" null null))
  (bind _output_get (set `self.Weapon` _returnvalue))
  (`self.K2_AttachToComponent` _output_get (`self.SkeletalMesh`) "Weapon_R" "SnapToTarget" "SnapToTarget" "SnapToTarget" true)
  (bind _asctr_aicontroller (cast `/Game/01_FriendlyAI/CTR_AIController` (`AIBlueprintHelperLibrary.GetAIController` self))
    (:`then`
      (set `/Game/01_FriendlyAI/CTR_AIController.AIPawn` self _asctr_aicontroller))
    (:`CastFailed`
      (`KismetSystemLibrary.PrintString` "Pawn_ControllerCastFail"))))

(event `self.ReceiveTick`
  (params (DeltaSeconds :type "Float (single-precision)"))
  (bind (_velocity_x _velocity_y) (`KismetMathLibrary.BreakVector` (`MovementComponent.Velocity` (`self.FloatingPawnMovement`))))
  (bind _returnvalue (`KismetMathLibrary.Conv_VectorToRotator` (`KismetMathLibrary.MakeVector` _velocity_x _velocity_y)))
  (if (!= _returnvalue (struct))
    (`self.K2_SetActorRotation` _returnvalue))
  (bind _asctr_aicontroller (cast `/Game/01_FriendlyAI/CTR_AIController` (`self.GetController`)))
  (if (and (`self.HasTarget`) (not (`/Game/01_FriendlyAI/CTR_AIController.NeedMove` _asctr_aicontroller)))
    (`self.AimTarget`)))

(event `Fire`
  (bind _target (`self.Target`))
  (bind _weapon (`self.Weapon`))
  (bind _weapon_2 (`self.Weapon`))
  (bind _weapon_3 (`self.Weapon`))
  (bind _haveammo (`/Game/02_Gun/BP_WeaponBase.HaveAmmo` _weapon))
  (if (and (not (`/Game/02_Gun/BP_WeaponBase.DoReload` _weapon)) (`/Game/02_Gun/BP_WeaponBase.Can Fire` _weapon) _haveammo (`self.HasTarget`))
    (set `/Game/02_Gun/BP_WeaponBase.DoFire` true _weapon_3)
    (`/Engine/EditorBlueprintResources/StandardMacros.IsValid` _target
      (:`Is Valid`
        (`/Game/02_Gun/BP_WeaponBase.Fire` (`self.Weapon`) _target)
        (`|PlayMontage` (`self.SkeletalMesh`) "/Game/02_Gun/Riffle/Fire_Rifle_Hip_Montage.Fire_Rifle_Hip_Montage"))
      (:`Is Not Valid`
        (`KismetSystemLibrary.PrintString` "NoTarget")))
    (elif _haveammo
      (set `/Game/02_Gun/BP_WeaponBase.DoFire` false _weapon_3)
      (else
        (set `/Game/02_Gun/BP_WeaponBase.DoFire` false _weapon_3)
        (if (`self.IsCanReload`)
          (`|PlayMontage` (`self.SkeletalMesh`) "/Game/02_Gun/Riffle/Reload_Rifle_Motage.Reload_Rifle_Motage"
            (:`OnCompleted`
              (`/Game/02_Gun/BP_WeaponBase.Reload` _weapon_2)
              (set `/Game/02_Gun/BP_WeaponBase.DoReload` false _weapon_2))))))))

(fn `AimTarget`
  (bind _target (`self.Target`))
  (bind (_returnvalue_roll _returnvalue_pitch _returnvalue_yaw) (`KismetMathLibrary.BreakRotator` (`KismetMathLibrary.FindLookAtRotation` (`self.K2_GetActorLocation`) (`self.K2_GetActorLocation` _target))))
  (`/Engine/EditorBlueprintResources/StandardMacros.IsValid` _target
    (:`Is Valid`
      (`self.K2_SetActorRotation` (`KismetMathLibrary.MakeRotator` _returnvalue_roll 0.0 _returnvalue_yaw))
      (set `self.SetAimSpace` (* _returnvalue_pitch -1.0)))))

(fn `Die`
  (`GameplayStatics.SpawnEmitterAtLocation` "/Game/StarterContent/Particles/P_Explosion.P_Explosion" (`self.K2_GetActorLocation`) (struct) (3.0 3.0 3.0))
  (`self.K2_DestroyActor` (`self.Weapon`))
  (`self.K2_DestroyActor`))

(fn `IsCanReload`
  (returns (CanReload :type Boolean))
  (bind _weapon (`self.Weapon`))
  (bind _weapon_2 (`self.Weapon`))
  (if (and (`/Game/02_Gun/BP_WeaponBase.HaveTotalAmmo` _weapon) (not (`/Game/02_Gun/BP_WeaponBase.DoReload` _weapon)) (!= (`/Game/02_Gun/BP_WeaponBase.CurrentAmmo` _weapon) (`/Game/02_Gun/BP_WeaponBase.MaxMagAmmo` _weapon)))
    (set `/Game/02_Gun/BP_WeaponBase.DoReload` true _weapon_2)
    (set `/Game/02_Gun/BP_WeaponBase.Can Fire` false _weapon_2)
    (return true)
    (else
      (return false))))

(fn `UserConstructionScript`)