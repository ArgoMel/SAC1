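; Base weapon Blueprint that fires hitscan shots at a target actor and tracks magazine and reserve ammo.
; Fire spends a round, line-traces from the MuzzleFlash socket to the target's location with debug drawing, and damages the hit actor, or calls Reload when empty.
; CanFire clears after each shot and returns after a delay if ammo remains, though Fire never checks it.
; Reload refills from reserve, which GetAmmo increases.
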(event `Shot Delay`
  (`KismetSystemLibrary.Delay` (`self.ShotDelay`))
  (if (`self.HaveAmmo`)
    (set `self.Can Fire` true)))

(fn `Fire`
  (params (Target :type "Actor Object Reference"))
  (if (`self.HaveAmmo`)
    (`|ExecutionSequence`
      (:`then_0`
        (bind _output_get (set `self.CurrentAmmo` (- (`self.CurrentAmmo`) 1)))
        (set `self.HaveAmmo` (> _output_get 0))
        (set `self.Can Fire` false)
        (`self.Shot Delay`))
      (:`then_1`
        (bind _outhit (`KismetSystemLibrary.LineTraceSingle` :`Start` (`SceneComponent.GetSocketLocation` (`self.SkeletalMesh`) "MuzzleFlash") :`End` (`self.K2_GetActorLocation` Target) :`TraceChannel` "TraceTypeQuery5" :`DrawDebugType` "ForOneFrame" :`DrawTime` 2.0))
        (`GameplayStatics.ApplyDamage` (`.HitActor` (`GameplayStatics.BreakHitResult` _outhit)) (`self.Damage`))))
    (else
      (`self.Reload`))))

(fn `GetAmmo`
  (params (AddAmmo :type Integer))
  (set `self.CurrentTotalAmmo` (+ AddAmmo (`self.CurrentTotalAmmo`))))

(fn `Reload`
  (bind _returnvalue (- (`self.MaxMagAmmo`) (`self.CurrentAmmo`)))
  (if (>= (`self.CurrentTotalAmmo`) _returnvalue)
    (set `self.CurrentTotalAmmo` (- (`self.CurrentTotalAmmo`) _returnvalue))
    (set `self.CurrentAmmo` (`self.MaxMagAmmo`))
    (else
      (set `self.CurrentAmmo` (+ (`self.CurrentTotalAmmo`) (`self.CurrentAmmo`)))
      (set `self.CurrentTotalAmmo` 0)))
  (set `self.HaveTotalAmmo` (> (`self.CurrentTotalAmmo`) 0))
  (set `self.HaveAmmo` true)
  (set `self.Can Fire` true))

(fn `UserConstructionScript`)